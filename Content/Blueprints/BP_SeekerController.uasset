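; AI controller for the Seeker that reacts to spotting and losing Hider characters.
; On BeginPlay it runs BT_Seeker and caches the controlled BP_Seeker pawn.
; AI Perception updates feed the Blackboard: a sensed Hider sets the target location, target actor and alert flag, and raises the Seeker's walk speed.
; Losing a Hider clears the target and alert flag and lowers speed, leaving the last stimulus location in place.
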(event `self.ReceiveBeginPlay`
  (`self.RunBehaviorTree` "/Game/AI/BT_Seeker.BT_Seeker")
  (bind _asbp_seeker (cast `/Game/Blueprints/BP_Seeker` (`self.K2_GetPawn`)))
  (set `self.As BP Seeker` _asbp_seeker))

(event `self.AIPerception.OnTargetPerceptionUpdated`
  (params (Actor :type "Actor Object Reference") (Stimulus :type "AIStimulus Structure"))
  (bind (_age _expirationage _strength _stimuluslocation _receiverlocation _tag _bsuccessfullysensed) (break `AIStimulus` Stimulus))
  (if (`KismetMathLibrary.ClassIsChildOf` (`GameplayStatics.GetObjectClass` Actor) "/Game/Blueprints/BP_Hider.BP_Hider_C")
    (if _bsuccessfullysensed
      (`KismetSystemLibrary.PrintString` "SEE HIDER")
      (`BlackboardComponent.SetValueAsVector` (`self.Blackboard`) "TargetLocation" _stimuluslocation)
      (`BlackboardComponent.SetValueAsBool` (`self.Blackboard`) "IsAlert" true)
      (`BlackboardComponent.SetValueAsObject` (`self.Blackboard`) "TargetHider" Actor)
      (set `CharacterMovementComponent.MaxWalkSpeed` 2000.0 (`Character.CharacterMovement` (`self.As BP Seeker`)))
      (else
        (`KismetSystemLibrary.PrintString` "CANNOT SEE HIDER")
        (`BlackboardComponent.SetValueAsObject` (`self.Blackboard`) "TargetHider" null)
        (set `CharacterMovementComponent.MaxWalkSpeed` 1000.0 (`Character.CharacterMovement` (`self.As BP Seeker`)))
        (`BlackboardComponent.SetValueAsBool` (`self.Blackboard`) "IsAlert" false)))))

(fn `UserConstructionScript`)