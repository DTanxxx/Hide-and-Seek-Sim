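; BP_Hider is a player character moved by holding the left mouse button, with the cursor shown on play.
; The button opens and closes a gate on Tick, so the move destination updates every frame while held.
; Each update traces the Visibility channel under the cursor and calls SimpleMoveToLocation on the player controller.
; Walk speed is raised when the destination is far from the character and lowered when it is close.
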(event `self.ReceiveBeginPlay`
  (set `PlayerController.bShowMouseCursor` true (`GameplayStatics.GetPlayerController` 0)))

(event `self.ReceiveTick`
  (params (DeltaSeconds :type "Float (single-precision)"))
  (`/Engine/EditorBlueprintResources/StandardMacros.Gate` true :!label _label
    (:`Exit`
      (`self.MoveToClickedPoint`))))

(event `Key|LeftMouseButton`
  (params (Key :type "Key Structure"))
  (:`Pressed`
    (goto _label :!via `Open`))
  (:`Released`
    (goto _label :!via `Close`)))

(fn `GetDestinationToMove`
  (returns (Destination :type "Vector Structure"))
  (return (`.Location` (`GameplayStatics.BreakHitResult` (`PlayerController.GetHitResultUnderCursorByChannel` (`GameplayStatics.GetPlayerController` 0) "TraceTypeQuery1" true)))))

(fn `MoveToClickedPoint`
  (locals (MoveDestination :type "Vector Structure"))
  (bind _charactermovement (`self.CharacterMovement`))
  (bind _destination (`self.GetDestinationToMove`))
  (set `local.MoveDestination` _destination)
  (if (> (`KismetMathLibrary.VSize` (- (`local.MoveDestination`) (`self.K2_GetActorLocation`))) 150.0)
    (set `CharacterMovementComponent.MaxWalkSpeed` 1500.0 _charactermovement)
    (else
      (set `CharacterMovementComponent.MaxWalkSpeed` 1000.0 _charactermovement)))
  (`AIBlueprintHelperLibrary.SimpleMoveToLocation` (`GameplayStatics.GetPlayerController` 0) (`local.MoveDestination`)))

(fn `UserConstructionScript`)