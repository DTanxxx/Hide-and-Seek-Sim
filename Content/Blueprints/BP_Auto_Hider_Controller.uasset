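; AI controller for the auto hider in a hide-and-seek game, running the BT_Hider behavior tree on its pawn.
; Perceiving a seeker sets alert blackboard keys, picks a random reachable flee point away from it, and boosts speed; losing it clears the alert and slows.
; Tick destroys the hider when the last seen seeker comes within catch range.
; A helper returns the nearest tagged hiding spot from those gathered at BeginPlay.
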(event `self.ReceiveBeginPlay`
  (bind _outactors (`GameplayStatics.GetAllActorsWithTag` "HidingSpot"))
  (set `self.HidingSpots` _outactors)
  (bind _asbp_auto_hider (cast `/Game/Blueprints/BP_Auto_Hider` (`self.K2_GetPawn`)))
  (set `self.As BP Auto Hider` _asbp_auto_hider)
  (`self.RunBehaviorTree` "/Game/AI/BT_Hider.BT_Hider"))

(event `self.ReceiveTick`
  (params (DeltaSeconds :type "Float (single-precision)"))
  (if (`KismetSystemLibrary.IsValid` (`self.Seeker`))
    (if (<= (`KismetMathLibrary.Vector_Distance` (`self.K2_GetActorLocation` (`self.Seeker`)) (`self.K2_GetActorLocation` (`self.As BP Auto Hider`))) 400.0)
      (`self.K2_DestroyActor` (`self.As BP Auto Hider`)))))

(event `self.AIPerception.OnTargetPerceptionUpdated`
  (params (Actor :type "Actor Object Reference") (Stimulus :type "AIStimulus Structure"))
  (bind (_age _expirationage _strength _stimuluslocation _receiverlocation _tag _bsuccessfullysensed) (break `AIStimulus` Stimulus))
  (bind _returnvalue (`self.K2_GetActorLocation` (`self.As BP Auto Hider`)))
  (if (`KismetMathLibrary.ClassIsChildOf` (`GameplayStatics.GetObjectClass` Actor) "/Game/Blueprints/BP_Seeker.BP_Seeker_C")
    (if _bsuccessfullysensed
      (set `self.Seeker` Actor)
      (`KismetSystemLibrary.PrintString` "SEE SEEKER")
      (`BlackboardComponent.SetValueAsVector` (`self.Blackboard`) "TargetLocation" (`NavigationSystemV1.K2_GetRandomReachablePointInRadius` (+ (* (`KismetMathLibrary.Normal` (- _returnvalue _stimuluslocation)) 2500.0) _returnvalue) 1000.0 null null))
      (`BlackboardComponent.SetValueAsBool` (`self.Blackboard`) "IsAlert" true)
      (`BlackboardComponent.SetValueAsObject` (`self.Blackboard`) "TargetSeeker" Actor)
      (set `CharacterMovementComponent.MaxWalkSpeed` 5000.0 (`Character.CharacterMovement` (`self.As BP Auto Hider`)))
      (else
        (`KismetSystemLibrary.PrintString` "CANNOT SEE SEEKER")
        (`BlackboardComponent.SetValueAsObject` (`self.Blackboard`) "TargetSeeker" null)
        (set `CharacterMovementComponent.MaxWalkSpeed` 2000.0 (`Character.CharacterMovement` (`self.As BP Auto Hider`)))
        (`BlackboardComponent.SetValueAsBool` (`self.Blackboard`) "IsAlert" false)))))

(fn `GetNearestHidingSpot`
  (returns (result :type "Actor Object Reference"))
  (locals (closest :type "Actor Object Reference"))
  (bind _hidingspots (`self.HidingSpots`))
  (set `local.closest` (`|GetArrayItem` _hidingspots))
  (for (_array_element _array_index) _hidingspots
    (if (!= _array_index 0)
      (if (< (`self.GetDistanceTo` _array_element (`self.As BP Auto Hider`)) (`self.GetDistanceTo` (`local.closest`) (`self.As BP Auto Hider`)))
        (set `local.closest` _array_element))))
  (return (`local.closest`)))

(fn `UserConstructionScript`)